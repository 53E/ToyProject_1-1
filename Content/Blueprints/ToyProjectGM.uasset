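; Game mode that runs a five-wave monster spawner for the toy project.
; A looping timer calls the current wave's function while IsStart is set, spawning one monster per tick at a random SpawnPoint and switching monster type within mixed waves.
; Once the quota is spent and no monsters remain, it sets up the next wave and clears IsStart for a break.
; Wave 5, the large monster, repeats indefinitely.
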(event `self.ReceiveBeginPlay`
  (bind _outactors (`GameplayStatics.GetAllActorsOfClass` "/Game/Blueprints/SpawnPoint.SpawnPoint_C"))
  (set `self.SpawnPoint` _outactors)
  ;[0 0 0] Wave 1 Info
  (set `self.NumberOfRemainMonsters` 3)
  (`KismetSystemLibrary.K2_SetTimerDelegate` (delegate `Spawn`) 2.0 true))

(event `Spawn`
  (if (`self.IsStart?`)
    (switch `/Game/Blueprints/Enums/Wave` (`self.Wave`)
      (:`NewEnumerator0`
        (`self.Wave1`))
      (:`NewEnumerator1`
        (`self.Wave2`))
      (:`NewEnumerator2`
        (`self.Wave3`))
      (:`NewEnumerator3`
        (`self.Wave4`))
      (:`NewEnumerator4`
        (`self.Wave5`)))
    (else
      (`KismetSystemLibrary.PrintString` "breaktime"))))

(fn `UserConstructionScript`)

(fn `Wave1`
  (bind _spawnpoint (`self.SpawnPoint`))
  (if (> (`self.NumberOfRemainMonsters`) 0)
    (`/Game/Blueprints/SpawnPoint.SpawnMonster` (`|GetArrayItem` _spawnpoint (`KismetMathLibrary.RandomIntegerInRange` 0 (- (`KismetArrayLibrary.Array_Length` _spawnpoint) 1))) "/Game/Blueprints/Monsters/WalkingMonster_1.WalkingMonster_1_C")
    (`/Engine/EditorBlueprintResources/StandardMacros.IncrementInt` (`self.NumberOfCurMonsters`) ; 현재 몬스터 수 증가
      (:`  `
        (`/Engine/EditorBlueprintResources/StandardMacros.DecrementInt` (`self.NumberOfRemainMonsters`)) ; 소환해야할 남은 몬스터수 감소
      ))
    (elif (not (> (`self.NumberOfCurMonsters`) 0))
      (bind _outactors (`GameplayStatics.GetAllActorsOfClass` "/Game/Blueprints/Monsters/DefaultMonsterBP.DefaultMonsterBP_C"))
      (if (not (> (`KismetArrayLibrary.Array_Length` _outactors) 0))
        (`/Engine/EditorBlueprintResources/StandardMacros.IncrementInt` (`self.NumberOfWave`)
          (:`  `
            ;[0 0 0] Wave2 Info
            (set `self.Wave` "NewEnumerator1")
            (set `self.NumberOfRemainMonsters` 2) ; Wave2 Monster
            (set `self.IsStart?` false)
            (set `self.NumberOfCurMonsters` 0)))))))

(fn `Wave2`
  (bind _spawnpoint (`self.SpawnPoint`))
  (if (> (`self.NumberOfRemainMonsters`) 0)
    (`/Game/Blueprints/SpawnPoint.SpawnMonster` (`|GetArrayItem` _spawnpoint (`KismetMathLibrary.RandomIntegerInRange` 0 (- (`KismetArrayLibrary.Array_Length` _spawnpoint) 1))) "/Game/Blueprints/Monsters/RunningMonster_1.RunningMonster_1_C") ; 몬스터 종류
    (`/Engine/EditorBlueprintResources/StandardMacros.IncrementInt` (`self.NumberOfCurMonsters`) ; 현재 몬스터 수 증가
      (:`  `
        (`/Engine/EditorBlueprintResources/StandardMacros.DecrementInt` (`self.NumberOfRemainMonsters`)) ; 소환해야할 남은 몬스터수 감소
      ))
    (elif (not (> (`self.NumberOfCurMonsters`) 0))
      (bind _outactors (`GameplayStatics.GetAllActorsOfClass` "/Game/Blueprints/Monsters/DefaultMonsterBP.DefaultMonsterBP_C"))
      (if (not (> (`KismetArrayLibrary.Array_Length` _outactors) 0))
        (`/Engine/EditorBlueprintResources/StandardMacros.IncrementInt` (`self.NumberOfWave`)
          (:`  `
            ;[0 0 0] Wave 3 Info
            (set `self.Wave` "NewEnumerator2")
            (set `self.NumberOfRemainMonsters` 6) ; Wave3 Monster
            (set `self.Walking1` 3)
            (set `self.Running1` 3)
            (set `self.KindOfMonster` "NewEnumerator0")
            (set `self.IsStart?` false)
            (set `self.NumberOfCurMonsters` 0)))))))

(fn `Wave3`
  (bind _spawnpoint (`self.SpawnPoint`))
  (bind _output (`|GetArrayItem` _spawnpoint (`KismetMathLibrary.RandomIntegerInRange` 0 (- (`KismetArrayLibrary.Array_Length` _spawnpoint) 1))))
  ;[0 0 0] 남은 몬스터가 없고 현재 몬스터가 없다면 웨이브 클리어
  (if (> (`self.NumberOfRemainMonsters`) 0)
    (switch `/Game/Blueprints/Enums/Monsters` (`self.KindOfMonster`)
      (:`NewEnumerator0`
        (`/Game/Blueprints/SpawnPoint.SpawnMonster` _output "/Game/Blueprints/Monsters/WalkingMonster_1.WalkingMonster_1_C") ; 몬스터 종류
        (`/Engine/EditorBlueprintResources/StandardMacros.IncrementInt` (`self.NumberOfCurMonsters`) ; 현재 몬스터 수 증가
          (:`  `
            (`/Engine/EditorBlueprintResources/StandardMacros.DecrementInt` (`self.NumberOfRemainMonsters`) ; 소환해야할 남은 몬스터수 감소
              (:`  `
                (`/Engine/EditorBlueprintResources/StandardMacros.DecrementInt` (`self.Walking1`)
                  (:`  `
                    (if (<= (`self.Walking1`) 0)
                      (set `self.KindOfMonster` "NewEnumerator1")))))))))
      (:`NewEnumerator1`
        (`/Game/Blueprints/SpawnPoint.SpawnMonster` _output "/Game/Blueprints/Monsters/RunningMonster_1.RunningMonster_1_C") ; 몬스터 종류
        (`/Engine/EditorBlueprintResources/StandardMacros.IncrementInt` (`self.NumberOfCurMonsters`) ; 현재 몬스터 수 증가
          (:`  `
            (`/Engine/EditorBlueprintResources/StandardMacros.DecrementInt` (`self.NumberOfRemainMonsters`)) ; 소환해야할 남은 몬스터수 감소
          ))))
    (elif (not (> (`self.NumberOfCurMonsters`) 0))
      (bind _outactors (`GameplayStatics.GetAllActorsOfClass` "/Game/Blueprints/Monsters/DefaultMonsterBP.DefaultMonsterBP_C"))
      (if (not (> (`KismetArrayLibrary.Array_Length` _outactors) 0))
        (`/Engine/EditorBlueprintResources/StandardMacros.IncrementInt` (`self.NumberOfWave`)
          (:`  `
            ;[0 0 0] Wave4 Info
            (set `self.Wave` "NewEnumerator3")
            (set `self.NumberOfRemainMonsters` 3)
            (set `self.Wobbling1` 3)
            (set `self.KindOfMonster` "NewEnumerator2")
            (set `self.IsStart?` false)
            (set `self.NumberOfCurMonsters` 0)))))))

(fn `Wave4`
  (bind _spawnpoint (`self.SpawnPoint`))
  (if (> (`self.NumberOfRemainMonsters`) 0)
    (switch `/Game/Blueprints/Enums/Monsters` (`self.KindOfMonster`)
      (:`NewEnumerator2`
        (`/Game/Blueprints/SpawnPoint.SpawnMonster` (`|GetArrayItem` _spawnpoint (`KismetMathLibrary.RandomIntegerInRange` 0 (- (`KismetArrayLibrary.Array_Length` _spawnpoint) 1))) "/Game/Blueprints/Monsters/WobblingMonster_1.WobblingMonster_1_C") ; 몬스터 종류
        (`/Engine/EditorBlueprintResources/StandardMacros.IncrementInt` (`self.NumberOfCurMonsters`) ; 현재 몬스터 수 증가
          (:`  `
            (`/Engine/EditorBlueprintResources/StandardMacros.DecrementInt` (`self.NumberOfRemainMonsters`) ; 소환해야할 남은 몬스터수 감소
              (:`  `
                (`/Engine/EditorBlueprintResources/StandardMacros.DecrementInt` (`self.Wobbling1`)
                  (:`  `
                    (if (<= (`self.Wobbling1`) 0)
                      _)))))))))
    (elif (not (> (`self.NumberOfCurMonsters`) 0))
      (bind _outactors (`GameplayStatics.GetAllActorsOfClass` "/Game/Blueprints/Monsters/DefaultMonsterBP.DefaultMonsterBP_C"))
      (if (not (> (`KismetArrayLibrary.Array_Length` _outactors) 0))
        (set `self.Wave` "NewEnumerator4")
        (`/Engine/EditorBlueprintResources/StandardMacros.IncrementInt` (`self.NumberOfWave`)
          (:`  `
            (set `self.NumberOfRemainMonsters` 1)
            (set `self.Large1` 1)
            (set `self.KindOfMonster` "NewEnumerator3")
            (set `self.IsStart?` false)
            (set `self.NumberOfCurMonsters` 0)))))))

(fn `Wave5`
  (bind _spawnpoint (`self.SpawnPoint`))
  (if (> (`self.NumberOfRemainMonsters`) 0)
    (switch `/Game/Blueprints/Enums/Monsters` (`self.KindOfMonster`)
      (:`NewEnumerator3`
        (`/Game/Blueprints/SpawnPoint.SpawnMonster` (`|GetArrayItem` _spawnpoint (`KismetMathLibrary.RandomIntegerInRange` 0 (- (`KismetArrayLibrary.Array_Length` _spawnpoint) 1))) "/Game/Blueprints/Monsters/LargeMonster_1.LargeMonster_1_C") ; 몬스터 종류
        (`/Engine/EditorBlueprintResources/StandardMacros.IncrementInt` (`self.NumberOfCurMonsters`) ; 현재 몬스터 수 증가
          (:`  `
            (`/Engine/EditorBlueprintResources/StandardMacros.DecrementInt` (`self.NumberOfRemainMonsters`) ; 소환해야할 남은 몬스터수 감소
              (:`  `
                (`/Engine/EditorBlueprintResources/StandardMacros.DecrementInt` (`self.Large1`)
                  (:`  `
                    (if (<= (`self.Large1`) 0)
                      (set `self.KindOfMonster` "NewEnumerator0"))))))))))
    (elif (not (> (`self.NumberOfCurMonsters`) 0))
      (bind _outactors (`GameplayStatics.GetAllActorsOfClass` "/Game/Blueprints/Monsters/DefaultMonsterBP.DefaultMonsterBP_C"))
      (if (not (> (`KismetArrayLibrary.Array_Length` _outactors) 0))
        (set `self.Wave` "NewEnumerator4")
        (`/Engine/EditorBlueprintResources/StandardMacros.IncrementInt` (`self.NumberOfWave`)
          (:`  `
            (set `self.NumberOfRemainMonsters` 1)
            (set `self.Large1` 1)
            (set `self.KindOfMonster` "NewEnumerator3")
            (set `self.IsStart?` false)
            (set `self.NumberOfCurMonsters` 0)))))))