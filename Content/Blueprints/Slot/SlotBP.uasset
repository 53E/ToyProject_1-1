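; SlotBP is a clickable slot actor that opens a SlotWB widget for itself when selected.
; Cursor hover events on the Slot component swap its material between default and highlighted versions.
; A click, gated by CanSpawn, removes any existing top-level SlotWB widgets, then adds a new one to the viewport and passes this actor to it as EmptySlot.
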(event `self.Slot.OnBeginCursorOver`
  (params (TouchedComponent :type "PrimitiveComponent Object Reference"))
  (`PrimitiveComponent.SetMaterial` (`self.Slot`) 0 "/Game/Blueprints/Slot/OnSlotM.OnSlotM"))

(event `self.Slot.OnEndCursorOver`
  (params (TouchedComponent :type "PrimitiveComponent Object Reference"))
  (`PrimitiveComponent.SetMaterial` (`self.Slot`) 0 "/Game/Blueprints/Slot/DefaultSlotM.DefaultSlotM"))

(event `self.Slot.OnClicked`
  (params (TouchedComponent :type "PrimitiveComponent Object Reference") (ButtonPressed :type "Key Structure"))
  (if (`self.CanSpawn?`)
    (bind _foundwidgets (`WidgetBlueprintLibrary.GetAllWidgetsOfClass` "/Game/HUD/SlotWB.SlotWB_C"))
    (for _array_element _foundwidgets
      (`Widget.RemoveFromParent` _array_element))
    (bind _returnvalue (`|CreateWidget` "/Game/HUD/SlotWB.SlotWB_C"))
    (`UserWidget.AddToViewport` _returnvalue 0)
    (set `/Game/HUD/SlotWB.EmptySlot` self _returnvalue)))

(event `self.Slot.OnReleased`
  (params (TouchedComponent :type "PrimitiveComponent Object Reference") (ButtonReleased :type "Key Structure")))

(fn `UserConstructionScript`)