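; DefaultTowerSlotBP is a tower slot actor that signals when the player stands within its overlap area.
; On BeginPlay it caches the hidden overlap widget, the ToyProjectGM game mode and the player character.
; Player entry shows the widget and sets CanPressVB on the game mode.
; Any end overlap, without an actor check, hides the widget and clears that flag.
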(event `self.ReceiveBeginPlay`
  (bind _asoverlap_slot_wb (cast `/Game/HUD/SlotWB/OverlapSlotWB` (`WidgetComponent.GetUserWidgetObject` (`self.OverlapWidget`))))
  (bind _output_get (set `self.As Overlap Slot WB` _asoverlap_slot_wb))
  (`Widget.SetVisibility` _output_get "Hidden")
  (bind _astoy_project_gm (cast `/Game/Blueprints/ToyProjectGM` (`GameplayStatics.GetGameMode`)))
  (set `self.As Toy Project GM` _astoy_project_gm)
  (bind _asplayer_bp (cast `/Game/Blueprints/Player/PlayerBP` (`GameplayStatics.GetPlayerCharacter` 0)))
  (set `self.As Player BP` _asplayer_bp))

(event `self.Overlap.OnComponentBeginOverlap`
  (params (OverlappedComponent :type "PrimitiveComponent Object Reference") (OtherActor :type "Actor Object Reference") (OtherComp :type "PrimitiveComponent Object Reference") (OtherBodyIndex :type Integer) (bFromSweep :type Boolean) (SweepResult :type "HitResult Structure (by ref)"))
  (cast `/Game/Blueprints/Player/PlayerBP` OtherActor)
  (`Widget.SetVisibility` (`self.As Overlap Slot WB`) "Visible")
  (set `/Game/Blueprints/ToyProjectGM.CanPress_V_B` true (`self.As Toy Project GM`)))

(event `self.Overlap.OnComponentEndOverlap`
  (params (OverlappedComponent :type "PrimitiveComponent Object Reference") (OtherActor :type "Actor Object Reference") (OtherComp :type "PrimitiveComponent Object Reference") (OtherBodyIndex :type Integer))
  (`Widget.SetVisibility` (`self.As Overlap Slot WB`) "Hidden")
  (set `/Game/Blueprints/ToyProjectGM.CanPress_V_B` false (`self.As Toy Project GM`)))

(fn `UserConstructionScript`)