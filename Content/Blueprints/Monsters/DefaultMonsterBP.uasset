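; Base monster Blueprint that walks to the first Goal actor, retrying on failure, and despawns on arrival.
; A health bar widget receives a reference to the monster at spawn.
; Damage reduces Hp; death runs once, disabling collision and movement, playing a boss (Large) or random montage, then a particle before destruction.
; Both arrival and death decrement ToyProjectGM's live monster count; SpeedMove doubles as walk speed and acceptance radius.
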(event `self.ReceiveBeginPlay`
  (`|ExecutionSequence`
    (:`then_0`
      (`self.GoToGoal`))
    (:`then_1`
      (bind _asdefault_monster_hpwb (cast `/Game/HUD/HP/DefaultMonsterHPWB` (`WidgetComponent.GetUserWidgetObject` (`self.MonsterHP`))))
      (set `/Game/HUD/HP/DefaultMonsterHPWB.DefaultMonster` self _asdefault_monster_hpwb))))

(event `GoToGoal`
  (`KismetSystemLibrary.Delay` 0.1)
  (set `CharacterMovementComponent.MaxWalkSpeed` (`self.speedMove`) (`self.CharacterMovement`))
  (bind _outactors (`GameplayStatics.GetAllActorsOfClass` "/Game/Blueprints/Goal.Goal_C"))
  (`|AIMoveTo` self (0.0 0.0 0.0) (`|GetArrayItem` _outactors) (`self.speedMove`)
    (:`OnSuccess`
      (`self.K2_DestroyActor`)
      (bind _astoy_project_gm (cast `/Game/Blueprints/ToyProjectGM` (`GameplayStatics.GetGameMode`)))
      (bind _output_get (set `self.As Toy Project GM` _astoy_project_gm))
      (`/Engine/EditorBlueprintResources/StandardMacros.DecrementInt` (`/Game/Blueprints/ToyProjectGM.NumberOfCurMonsters` _output_get)))
    (:`OnFail`
      (`self.GoToGoal`))))

(event `self.ReceiveAnyDamage`
  (params (Damage :type "Float (single-precision)") (DamageType :type "DamageType Object Reference") (InstigatedBy :type "Controller Object Reference") (DamageCauser :type "Actor Object Reference"))
  (set `self.Hp` (- (`self.Hp`) Damage))
  (if (<= (`self.Hp`) 0.0)
    (if (`self.HPGood?`)
      (set `self.HPGood?` false) ; death
      (`SceneComponent.SetVisibility` (`self.MonsterHP`) false false)
      (`PrimitiveComponent.SetCollisionEnabled` (`self.CapsuleComponent`) "NoCollision")
      (set `CharacterMovementComponent.MaxWalkSpeed` 0.0 (`self.CharacterMovement`))
      (bind _astoy_project_gm (cast `/Game/Blueprints/ToyProjectGM` (`GameplayStatics.GetGameMode`)))
      (`/Engine/EditorBlueprintResources/StandardMacros.DecrementInt` (`/Game/Blueprints/ToyProjectGM.NumberOfCurMonsters` _astoy_project_gm)
        (:`  `
          (if (`self.Large?`)
            (`self.PlayAnimMontage` "/Game/Blueprints/Anims/anim/MonsterDeathAnim/Death_Large1.Death_Large1")
            (`KismetSystemLibrary.Delay` 2.0)
            (else
              (`self.PlayAnimMontage` (select `int` (`KismetMathLibrary.RandomIntegerInRange` 0 3) :`0` (`self.DeathAnim_1`) :`1` (`self.DeathAnim_2`) :`2` (`self.DeathAnim_3`) :`3` (`self.DeathAnim_4`)))
              (`KismetSystemLibrary.Delay` 2.0)))
          (bind _returnvalue (`GameplayStatics.SpawnEmitterAtLocation` "/Game/Blueprints/Monsters/Particle/DeathParticle.DeathParticle" (`KismetMathLibrary.MakeVector` (.x (`self.K2_GetActorLocation`)) (.y (`self.K2_GetActorLocation`)) (- (.z (`self.K2_GetActorLocation`)) 75.0)) (struct) (0.15 0.15 0.15)))
          (`KismetSystemLibrary.Delay` 0.8)
          (`ActorComponent.Deactivate` _returnvalue)
          (`self.K2_DestroyActor`))))))

(fn `UserConstructionScript`)