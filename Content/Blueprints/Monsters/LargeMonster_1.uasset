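; Large monster Blueprint variant built on a parent monster class.
; On BeginPlay it sets its move speed, health and large flag.
; It then hands itself to the LargeMonsterHPWB health bar widget on its MonsterHP component and runs the parent BeginPlay only if that cast succeeds.
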(event `self.ReceiveBeginPlay`
  (set `self.speedMove` 40.0)
  (bind _output_get (set `self.MaxHP` 2500.0))
  (set `self.Hp` _output_get)
  (set `self.Large?` true)
  (bind _aslarge_monster_hpwb (cast `/Game/HUD/HP/LargeMonsterHPWB` (`WidgetComponent.GetUserWidgetObject` (`self.MonsterHP`))))
  (set `/Game/HUD/HP/LargeMonsterHPWB.DefaultMonster` self _aslarge_monster_hpwb)
  (`parent.ReceiveBeginPlay`))

(fn `UserConstructionScript`
  (`parent.UserConstructionScript`))