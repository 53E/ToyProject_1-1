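; Tower-defense tower actor that targets and fires at DefaultMonsterBP actors inside its Overlap component.
; Overlap events maintain an in-range array, from which a random target is picked when none is held.
; A gated, Delay-driven loop yaws the Tower toward the target and spawns InputBullet at the Sphere after RateOfShot, destroying it shortly afterwards.
; ResetAim is empty; the rotation-reset logic is disconnected.
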(event `ContinueAim`
  (bind _detectedmonster (`self.DetectedMonster`))
  (`/Engine/EditorBlueprintResources/StandardMacros.IsValid` _detectedmonster
    (:`Is Valid`
      (if (`/Game/Blueprints/Monsters/DefaultMonsterBP.HPGood?` _detectedmonster)
        (`/Engine/EditorBlueprintResources/StandardMacros.Gate` true :!label _label
          (:`Exit`
            (`/Engine/EditorBlueprintResources/StandardMacros.IsValid` (`self.DetectedMonster`)
              (:`Is Valid`
                (`|ExecutionSequence`
                  (:`then_0`
                    ;[0 0 0] Fire
                    (`KismetSystemLibrary.Delay` (`self.RateOfShot`))
                    (bind _bullet (`self.Shot` self (`self.Input Bullet`)))
                    (`KismetSystemLibrary.Delay` 0.4)
                    (`/Engine/EditorBlueprintResources/StandardMacros.IsValid` _bullet
                      (:`Is Valid`
                        (`self.K2_DestroyActor` _bullet))))
                  (:`then_1`
                    (set `self.TargetLocation` (`self.K2_GetActorLocation` (`self.DetectedMonster`)))
                    (`SceneComponent.K2_SetRelativeRotation` (`self.tower`) (`KismetMathLibrary.RInterpTo_Constant` (`SceneComponent.RelativeRotation` (`self.tower`)) (`KismetMathLibrary.MakeRotator` 0.0 0.0 (.yaw (`KismetMathLibrary.MakeRotFromX` (`KismetMathLibrary.InverseTransformDirection` (`self.GetTransform`) (- (`self.TargetLocation`) (`SceneComponent.K2_GetComponentLocation` (`self.tower`))))))) (`GameplayStatics.GetWorldDeltaSeconds`) (`self.Interp Speed`)) false false)
                    (`KismetSystemLibrary.Delay` (`GameplayStatics.GetWorldDeltaSeconds`))
                    (`self.ContinueAim`))))
              (:`Is Not Valid`
                (`self.CancleAim` :!label _label_2)
                (`self.ResetAim`)))))))
    (:`Is Not Valid`
      (`self.CancleAim`)
      (goto _label_2))))

(event `BeginAim`
  (`|ExecutionSequence`
    (:`then_0`
      (goto _label :!via `Open`))
    (:`then_1`
      (goto _label))))

(event `SelectTarget`
  (bind _targetinrange (`self.TargetInRange`))
  ;[0 0 0] 배열속 몬스터 랜덤 선택
  (if (`KismetArrayLibrary.Array_IsValidIndex` _targetinrange)
    (set `self.DetectedMonster` (`|GetArrayItem` _targetinrange (`KismetMathLibrary.RandomIntegerInRange` 0 (`KismetArrayLibrary.Array_LastIndex` _targetinrange))))
    (`self.BeginAim`)
    (else
      (`self.ResetAim`))))

(event `CancleAim`
  (goto _label :!via `Close`))

(event `self.Overlap.OnComponentBeginOverlap`
  (params (OverlappedComponent :type "PrimitiveComponent Object Reference") (OtherActor :type "Actor Object Reference") (OtherComp :type "PrimitiveComponent Object Reference") (OtherBodyIndex :type Integer) (bFromSweep :type Boolean) (SweepResult :type "HitResult Structure (by ref)"))
  ;[0 0 0] 범위 안에 들어올 시 배열에 몬스터 추가
  (bind _asdefault_monster_bp (cast `/Game/Blueprints/Monsters/DefaultMonsterBP` OtherActor))
  (`KismetArrayLibrary.Array_Add` (`self.TargetInRange`) _asdefault_monster_bp)
  (`/Engine/EditorBlueprintResources/StandardMacros.IsValid` (`self.DetectedMonster`)
    (:`Is Not Valid`
      (`self.SelectTarget`))))

(event `ContinueReset`)

(event `self.Overlap.OnComponentEndOverlap`
  (params (OverlappedComponent :type "PrimitiveComponent Object Reference") (OtherActor :type "Actor Object Reference") (OtherComp :type "PrimitiveComponent Object Reference") (OtherBodyIndex :type Integer))
  (bind _targetinrange (`self.TargetInRange`))
  ;[0 0 0] 범위 안에 들어올 시 배열에 몬스터 추가
  (bind _asdefault_monster_bp (cast `/Game/Blueprints/Monsters/DefaultMonsterBP` OtherActor))
  (if (`KismetArrayLibrary.Array_Contains` _targetinrange _asdefault_monster_bp)
    (`KismetArrayLibrary.Array_RemoveItem` _targetinrange _asdefault_monster_bp)
    (if (== _asdefault_monster_bp (`self.DetectedMonster`))
      (set `self.DetectedMonster` null)
      (`self.SelectTarget`))))

(event `ResetAim`)

(event `StopReset`)

(fn `Shot`
  (params (inputBullet :type "/Game/Blueprints/Tower/Bullet/DefaultBulletBP Class Reference"))
  (returns (Bullet :type "/Game/Blueprints/Tower/Bullet/DefaultBulletBP Object Reference"))
  (bind _returnvalue (`|SpawnActorFromClass` inputBullet (`SceneComponent.K2_GetComponentToWorld` (`self.Sphere`)) "Undefined" "OverrideRootScale" null null))
  (return _returnvalue))

(fn `UserConstructionScript`)