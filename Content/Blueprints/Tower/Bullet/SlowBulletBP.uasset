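; Slow-effect tower bullet Blueprint that damages what it overlaps and slows monsters that are not large.
; On overlap it sets its Damage, defers to the parent's overlap logic, then casts the other actor to DefaultMonsterBP.
; For non-large monsters it sets MaxWalkSpeed to a fraction of SpeedMove and raises the Slow flag, with no speed restore in this Blueprint.
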(event `self.ReceiveActorBeginOverlap`
  (params (OtherActor :type "Actor Object Reference"))
  (`|ExecutionSequence`
    (:`then_0`
      (set `self.Damage` 10.0)
      (`parent.ReceiveActorBeginOverlap` OtherActor))
    (:`then_1`
      (bind _asdefault_monster_bp (cast `/Game/Blueprints/Monsters/DefaultMonsterBP` OtherActor))
      (if (not (`/Game/Blueprints/Monsters/DefaultMonsterBP.Large?` _asdefault_monster_bp))
        (set `self.InitialSpeed` (`/Game/Blueprints/Monsters/DefaultMonsterBP.speedMove` _asdefault_monster_bp))
        (set `CharacterMovementComponent.MaxWalkSpeed` (/ (`self.InitialSpeed`) 5.0) (`Character.CharacterMovement` _asdefault_monster_bp))
        (set `/Game/Blueprints/Monsters/DefaultMonsterBP.Slow?` true _asdefault_monster_bp)))))

(fn `UserConstructionScript`
  (`parent.UserConstructionScript`))