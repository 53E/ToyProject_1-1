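; ToyPlayer is the player Blueprint for the Toy project, handling a start key and a mouse cursor toggle.
; On BeginPlay it caches the ToyProjectGM game mode, and pressing P sets that game mode's IsStart flag once.
; Pressing O flips the cursor, click and mouse-over events on player controller 0, calling DisableInput when the cursor appears and EnableInput when it hides.
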(event `self.ReceiveBeginPlay`
  (bind _astoy_project_gm (cast `/Game/Blueprints/ToyProjectGM` (`GameplayStatics.GetGameMode`)))
  (set `self.As Toy Project GM` _astoy_project_gm))

(event `InputAction|Press P`
  (params (Key :type "Key Structure"))
  (bind _as_toy_project_gm (`self.As Toy Project GM`))
  (:`Pressed`
    (if (not (`/Game/Blueprints/ToyProjectGM.IsStart?` _as_toy_project_gm))
      (set `/Game/Blueprints/ToyProjectGM.IsStart?` true _as_toy_project_gm))))

(event `InputAction|Press O`
  (params (Key :type "Key Structure"))
  (bind _returnvalue (`GameplayStatics.GetPlayerController` 0))
  (bind _returnvalue_2 (`GameplayStatics.GetPlayerController` 0))
  (:`Pressed`
    (if (`self.Mouse?`)
      (set `PlayerController.bShowMouseCursor` false _returnvalue)
      (set `PlayerController.bEnableClickEvents` false _returnvalue)
      (set `PlayerController.bEnableMouseOverEvents` false _returnvalue)
      (set `self.Mouse?` false)
      (`self.EnableInput` _returnvalue_2 null)
      (else
        (set `PlayerController.bShowMouseCursor` true _returnvalue)
        (set `PlayerController.bEnableClickEvents` true _returnvalue)
        (set `PlayerController.bEnableMouseOverEvents` true _returnvalue)
        (set `self.Mouse?` true)
        (`self.DisableInput` _returnvalue_2 null)))))

(fn `UserConstructionScript`)