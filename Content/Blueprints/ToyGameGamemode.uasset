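; Wave-spawner game mode that sends walking and running monsters from random spawn points.
; PopulateMap reads each wave's per-type counts from WaveDetailTable into a map and a running total.
; A looping timer spawns a type picked by random retry, then stores the decremented total, not that type's count, in the map.
; Once none remain to spawn or alive, it prints "clear", waits, then loads the next wave.
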(event `self.ReceiveBeginPlay`
  (bind _outactors (`GameplayStatics.GetAllActorsOfClass` "/Game/Blueprints/SpawnPoint.SpawnPoint_C"))
  (set `self.list of spawn point` _outactors)
  (`KismetSystemLibrary.K2_SetTimerDelegate` (delegate `ActivateSpawn`) (`self.SpawnTime`) true)
  (`self.populate Map` (`self.WaveNumber`)))

(event `ActivateSpawn`
  (bind _list_of_spawn_point (`self.list of spawn point`))
  (if (> (`self.NumberOfMonster`) 0)
    (bind _newparam (`self.Choose Monster`))
    (`/Game/Blueprints/SpawnPoint.SpawnMonster` (`|GetArrayItem` _list_of_spawn_point (`KismetMathLibrary.RandomIntegerInRange` 0 (- (`KismetArrayLibrary.Array_Length` _list_of_spawn_point) 1))) _newparam)
    (else
      (bind _outactors (`GameplayStatics.GetAllActorsOfClass` "/Game/Blueprints/Monsters/DefaultMonsterBP.DefaultMonsterBP_C"))
      (if (<= (`KismetArrayLibrary.Array_Length` _outactors) 0)
        (`KismetSystemLibrary.PrintString` "clear")
        (`KismetSystemLibrary.Delay` 5.0)
        (bind _result (`/Engine/EditorBlueprintResources/StandardMacros.IncrementInt` (`self.WaveNumber`))
          (:`  `
            (`self.populate Map` _result)))))))

(fn `Choose Monster`
  (returns (NewParam :type "/Game/Blueprints/Monsters/DefaultMonsterBP Class Reference"))
  (bind _keys (`BlueprintMapLibrary.Map_Keys` (`self.MonsterList`) :!label _label))
  (bind _output_get (set `self.chosenMonster` (`|GetArrayItem` _keys (`KismetMathLibrary.RandomInteger` (`KismetArrayLibrary.Array_Length` _keys)))))
  (if (> (`BlueprintMapLibrary.Map_Find` (`self.MonsterList`) _output_get) 0)
    (`BlueprintMapLibrary.Map_Add` (`self.MonsterList`) (`self.chosenMonster`) (- (`self.NumberOfMonster`) 1))
    (set `self.NumberOfMonster` (- (`self.NumberOfMonster`) 1))
    (return (`self.chosenMonster`))
    (else
      (goto _label))))

(fn `populate Map`
  (params (WaveNumber :type Integer))
  (bind _returnvalue (`|GetDataTableRow` "/Game/Blueprints/Monsters/WaveDetailTable.WaveDetailTable" (`KismetStringLibrary.Conv_StringToName` (`KismetStringLibrary.Conv_IntToString` WaveNumber)))
    (:`then`
      (set `self.NumberOfAllMonster` (+ (break `/Game/Blueprints/Monsters/WaveDetailStruct` _returnvalue) (`.RunningMonster_8_1FE444904BF77DA3A78E0EAD99877490` (break `/Game/Blueprints/Monsters/WaveDetailStruct` _returnvalue))))
      (bind _output_get (set `self.MonsterList` (`|MakeMap` "/Game/Blueprints/Monsters/WalkingMonster_1.WalkingMonster_1_C" (break `/Game/Blueprints/Monsters/WaveDetailStruct` _returnvalue) "/Game/Blueprints/Monsters/RunningMonster_1.RunningMonster_1_C" (`.RunningMonster_8_1FE444904BF77DA3A78E0EAD99877490` (break `/Game/Blueprints/Monsters/WaveDetailStruct` _returnvalue)) :!type "/Game/Blueprints/Monsters/DefaultMonsterBP Class Reference")))
      (bind _values (`BlueprintMapLibrary.Map_Values` _output_get))
      (for _array_element _values
        (set `self.NumberOfMonster` (+ _array_element (`self.NumberOfMonster`)))))))

(fn `UserConstructionScript`)